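; BP_Bullet is a projectile that damages the side-scroller player and can be turned against AI characters.
; Hitting the player spawns attached Niagara effects, briefly shows the blood HUD, deducts fixed HP, destroys the player at zero and increments the game mode's hit count.
; The bullet destroys itself after that flash, or immediately on other hits.
; ChangeTeam marks it as reflected, so overlapping an AICharacter then spawns an explosion and destroys only the bullet.
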(event `self.Sphere.OnComponentHit`
  (params (HitComponent :type "PrimitiveComponent Object Reference") (OtherActor :type "Actor Object Reference") (OtherComp :type "PrimitiveComponent Object Reference") (NormalImpulse :type "Vector Structure") (Hit :type "HitResult Structure (by ref)"))
  (bind (_bblockinghit _binitialoverlap _time _distance _location _impactpoint _normal _impactnormal _physmat _hitactor _hitcomponent) (`GameplayStatics.BreakHitResult` Hit))
  (bind _returnvalue (== _hitactor (`GameplayStatics.GetPlayerPawn` 0)))
  (`|ExecutionSequence`
    (:`then_0`
      (if _returnvalue
        (bind _asside_scroller_character (cast `/Game/SideScrollerBP/Blueprints/SideScrollerCharacter` (`GameplayStatics.GetPlayerCharacter` 0)))
        (`NiagaraFunctionLibrary.SpawnSystemAttached` "/Game/AI/NewNiagaraEmitter_System.NewNiagaraEmitter_System" _hitcomponent "None" (0.0 0.0 0.0) (`KismetMathLibrary.Conv_VectorToRotator` _normal) "SnapToTarget" true)
        (bind _bloodhud (`/Game/SideScrollerBP/Blueprints/SideScrollerCharacter.BloodHud` _asside_scroller_character))
        (`Widget.SetVisibility` _bloodhud "Visible")
        (`KismetSystemLibrary.Delay` 0.5)
        (`Widget.SetVisibility` _bloodhud "Collapsed")
        (`self.K2_DestroyActor`)
        (else
          (`self.K2_DestroyActor`))))
    (:`then_1`
      (bind _asside_scroller_character_2 (cast `/Game/SideScrollerBP/Blueprints/SideScrollerCharacter` OtherActor))
      (bind _output_get (set `/Game/SideScrollerBP/Blueprints/SideScrollerCharacter.CurrentHP` (- (`/Game/SideScrollerBP/Blueprints/SideScrollerCharacter.CurrentHP` _asside_scroller_character_2) 10.0) _asside_scroller_character_2))
      (if (<= _output_get 0.0)
        (`Widget.SetVisibility` (`/Game/SideScrollerBP/Blueprints/SideScrollerCharacter.BloodHud` _asside_scroller_character_2) "Collapsed")
        (`self.K2_DestroyActor` (`GameplayStatics.GetPlayerCharacter` 0))))
    (:`then_2`
      (if _returnvalue
        (bind _asside_scroller_game_mode (cast `/Game/SideScrollerBP/Blueprints/SideScrollerGameMode` (`GameplayStatics.GetGameMode`)))
        (set `/Game/SideScrollerBP/Blueprints/SideScrollerGameMode.HitPlayerCount` (+ (`/Game/SideScrollerBP/Blueprints/SideScrollerGameMode.HitPlayerCount` _asside_scroller_game_mode) 1) _asside_scroller_game_mode)))))

(event `ChangeTeam`
  ;[1 1 1] Reflection projectile
  (set `self.damageParent` true))

(event `self.Sphere.OnComponentBeginOverlap`
  (params (OverlappedComponent :type "PrimitiveComponent Object Reference") (OtherActor :type "Actor Object Reference") (OtherComp :type "PrimitiveComponent Object Reference") (OtherBodyIndex :type Integer) (bFromSweep :type Boolean) (SweepResult :type "HitResult Structure (by ref)"))
  ;[1 1 1] Reflection projectile
  (if (`self.damageParent`)
    (cast `/Game/AI/AICharacter` OtherActor)
    (`GameplayStatics.SpawnEmitterAtLocation` "/Game/StarterContent/Particles/P_Explosion.P_Explosion" (`SceneComponent.K2_GetComponentLocation` (`self.Sphere`)))
    (`self.K2_DestroyActor`)))

(fn `UserConstructionScript`)