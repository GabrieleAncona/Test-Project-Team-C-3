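; Turret actor for a side-scroller that tracks and shoots at the player.
; Each tick, when the player is within range and an object line trace hits them, the head smoothly rotates toward them.
; A SpawnProjectile flag and delays pace the shots, showing an exclamation mesh before spawning a bullet with a sound.
; Tick also toggles the head's custom-depth outline from the player character's flag; older aiming logic remains unconnected.
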(event `self.ReceiveTick`
  (params (DeltaSeconds :type "Float (single-precision)"))
  (bind _turrethead (`self.TurretHead`))
  (`|ExecutionSequence`
    (:`then_0`
      (if (< (`KismetMathLibrary.VSize` (- (`self.K2_GetActorLocation` (`GameplayStatics.GetPlayerPawn` 0)) (`self.K2_GetActorLocation`))) (`self.Turret Trace Range`))
        (bind _outhit (`KismetSystemLibrary.LineTraceSingleForObjects` :`Start` (`self.K2_GetActorLocation`) :`End` (`self.K2_GetActorLocation` (`GameplayStatics.GetPlayerPawn` 0)) :`ObjectTypes` (`|MakeArray` "ObjectTypeQuery1" "ObjectTypeQuery3" :!type "EObjectTypeQuery Enum") :`DrawDebugType` "ForOneFrame"))
        (if (== (`GameplayStatics.GetPlayerPawn` 0) (`.HitActor` (`GameplayStatics.BreakHitResult` _outhit)))
          (bind _output_get (set `self.Actual Rotation` (`KismetMathLibrary.RInterpTo` (`self.Actual Rotation`) (`KismetMathLibrary.FindLookAtRotation` (`self.K2_GetActorLocation`) (`self.K2_GetActorLocation` (`GameplayStatics.GetPlayerPawn` 0))) (`GameplayStatics.GetWorldDeltaSeconds`) 8.0)))
          (`SceneComponent.K2_SetWorldRotation` (`self.TurretHead`) _output_get false false)
          (if (`self.SpawnProjectile`)
            (`SceneComponent.SetVisibility` (`self.Exclamation FBX turret`) true false)
            (`KismetSystemLibrary.Delay` (`self.shoot_delay`))
            (`|SpawnActorFromClass` "/Game/Developers/gabbo/BP_BulletDef.BP_BulletDef_C" (`SceneComponent.K2_GetComponentToWorld` (`self.ProjectileSpawnLocation`)) "Undefined" "OverrideRootScale" null null)
            (`GameplayStatics.PlaySound2D` "/Game/Sounds/GUN_FIRE-GoodSoundForYou-820112263.GUN_FIRE-GoodSoundForYou-820112263" 1.0 1.0 0.0 null null)
            (set `self.SpawnProjectile` false)
            (`SceneComponent.SetVisibility` (`self.Exclamation FBX turret`) false false)
            (`KismetSystemLibrary.Delay` (`self.shoot_delay`))
            (set `self.SpawnProjectile` true)))))
    (:`then_1`
      (bind _asside_scroller_character (cast `/Game/SideScrollerBP/Blueprints/SideScrollerCharacter` (`GameplayStatics.GetPlayerPawn` 0)))
      (if (`/Game/SideScrollerBP/Blueprints/SideScrollerCharacter.isOutlineTurret` _asside_scroller_character)
        (`PrimitiveComponent.SetRenderCustomDepth` _turrethead true)
        (`PrimitiveComponent.SetCustomDepthStencilValue` _turrethead 2)
        (else
          (`PrimitiveComponent.SetRenderCustomDepth` _turrethead false)
          (`PrimitiveComponent.SetCustomDepthStencilValue` _turrethead 0))))))

(fn `UserConstructionScript`)