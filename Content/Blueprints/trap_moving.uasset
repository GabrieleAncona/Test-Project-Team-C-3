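; A moving trap for a side-scroller that damages the player character on contact.
; On BeginPlay, a timeline lerps the static mesh's world location from the actor's start position toward that position offset by EndPoint.
; Box overlap subtracts Damage from the SideScrollerCharacter's CurrentHP and reopens the hardcoded SideScrollerExampleMap level when HP drops to zero or below.
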(event `self.Box.OnComponentBeginOverlap`
  (params (OverlappedComponent :type "PrimitiveComponent Object Reference") (OtherActor :type "Actor Object Reference") (OtherComp :type "PrimitiveComponent Object Reference") (OtherBodyIndex :type Integer) (bFromSweep :type Boolean) (SweepResult :type "HitResult Structure (by ref)"))
  (bind _asside_scroller_character (cast `/Game/SideScrollerBP/Blueprints/SideScrollerCharacter` OtherActor))
  (bind _output_get (set `/Game/SideScrollerBP/Blueprints/SideScrollerCharacter.CurrentHP` (- (`/Game/SideScrollerBP/Blueprints/SideScrollerCharacter.CurrentHP` _asside_scroller_character) (`self.Damage`)) _asside_scroller_character))
  (if (<= _output_get 0.0)
    (`GameplayStatics.OpenLevel` "SideScrollerExampleMap")))

(event `self.ReceiveBeginPlay`
  (set `self.Starting Point` (`self.K2_GetActorLocation`))
  (bind (_direction _newtrack_0) (`Timeline|Timeline_0`)
    (:`Update`
      (`SceneComponent.K2_SetWorldLocation` (`self.StaticMesh`) (`KismetMathLibrary.VLerp` (`self.Starting Point`) (+ (`self.Starting Point`) (`self.End Point`)) _newtrack_0) false false))))

(fn `UserConstructionScript`)