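; BP_ProceduralCorridor is a procedural corridor Blueprint that builds floor and wall geometry from repeated instanced meshes.
; The Construction Script applies floor and wall materials, then nested loops add one floor instance per horizontal segment, each with a vertical stack of wall instances.
; Running offsets step segments along negative Y and walls along Z, resetting height after each column.
; The event graph has no active logic.
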(fn `UserConstructionScript`
  (`PrimitiveComponent.SetMaterial` (`self.ISMC_Floor`) 0 (`self.FloorMat`))
  (`PrimitiveComponent.SetMaterial` (`self.ISMC_WallBase`) 0 (`self.WallMat`))
  (for _ (range 1 (+ (`self.HorizontalAmount`) 1))
    (`InstancedStaticMeshComponent.AddInstance` (`self.ISMC_Floor`) (`KismetMathLibrary.MakeTransform` (`KismetMathLibrary.MakeVector` 0.0 (`self.ActualOffsetHorizontal`))))
    (for _ (range 1 (+ (`self.VerticalAmount`) 1))
      (`InstancedStaticMeshComponent.AddInstance` (`self.ISMC_WallBase`) (`KismetMathLibrary.MakeTransform` (`KismetMathLibrary.MakeVector` 0.0 (`self.ActualOffsetHorizontal`) (`self.ActualOffsetVertical`))))
      (set `self.ActualOffsetVertical` (+ (`self.OffsetVertical`) (`self.ActualOffsetVertical`))))
    (set `self.ActualOffsetHorizontal` (- (`self.ActualOffsetHorizontal`) (`self.OffsetHorizontal`)))
    (set `self.ActualOffsetVertical` 0.0)))