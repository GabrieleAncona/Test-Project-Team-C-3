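; Procedural corridor building piece that assembles floor, walls and an optional roof from instanced static meshes in the Construction Script.
; Nested loops over horizontal and vertical counts step running offsets to tile a floor row and stacked base-wall grid, capping each column with a flipped roof tile when enabled.
; Optional left and right walls reuse those offsets along X, rotated 90 degrees either way.
; Each part takes its own material variable; the event graph is unused.
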(fn `UserConstructionScript`
  (`PrimitiveComponent.SetMaterial` (`self.ISMC_WallLeft`) 0 (`self.WallLMat`))
  (`PrimitiveComponent.SetMaterial` (`self.ISMC_WallRight`) 0 (`self.WallRMat`))
  (`PrimitiveComponent.SetMaterial` (`self.ISMC_Roof`) 0 (`self.RoofMat`))
  (`PrimitiveComponent.SetMaterial` (`self.ISMC_Floor`) 0 (`self.FloorMat`))
  (`PrimitiveComponent.SetMaterial` (`self.ISMC_WallBase`) 0 (`self.WallMat`))
  (for _ (range 1 (+ (`self.HorizontalAmount`) 1))
    (`InstancedStaticMeshComponent.AddInstance` (`self.ISMC_Floor`) (`KismetMathLibrary.MakeTransform` (`KismetMathLibrary.MakeVector` 0.0 (`self.ActualOffsetHorizontal`))))
    (for _ (range 1 (+ (`self.VerticalAmount`) 1))
      (`InstancedStaticMeshComponent.AddInstance` (`self.ISMC_WallBase`) (`KismetMathLibrary.MakeTransform` (`KismetMathLibrary.MakeVector` 0.0 (`self.ActualOffsetHorizontal`) (`self.ActualOffsetVertical`))))
      (`|ExecutionSequence`
        (:`then_0`
          (if (`self.HasWallLeft`)
            (`InstancedStaticMeshComponent.AddInstance` (`self.ISMC_WallLeft`) (`KismetMathLibrary.MakeTransform` (`KismetMathLibrary.MakeVector` (* (`self.ActualOffsetHorizontal`) -1.0) 0.0 (`self.ActualOffsetVertical`)) (struct :`Yaw` -90.0)))))
        (:`then_1`
          (if (`self.HasWallRight`)
            (`InstancedStaticMeshComponent.AddInstance` (`self.ISMC_WallRight`) (`KismetMathLibrary.MakeTransform` (`KismetMathLibrary.MakeVector` (* (`self.ActualOffsetHorizontal`) -1.0) 0.0 (`self.ActualOffsetVertical`)) (struct :`Yaw` 90.0)))))
        (:`then_2`
          (set `self.ActualOffsetVertical` (+ (`self.OffsetVertical`) (`self.ActualOffsetVertical`))))))
    (`|ExecutionSequence`
      (:`then_0`
        (if (`self.HasRoof`)
          (`InstancedStaticMeshComponent.AddInstance` (`self.ISMC_Roof`) (`KismetMathLibrary.MakeTransform` (`KismetMathLibrary.MakeVector` 0.0 (`self.ActualOffsetHorizontal`) (`self.ActualOffsetVertical`)) (struct :`Pitch` 180.0)))))
      (:`then_1`
        (set `self.ActualOffsetHorizontal` (- (`self.ActualOffsetHorizontal`) (`self.OffsetHorizontal`)))
        (set `self.ActualOffsetVertical` 0.0)))))