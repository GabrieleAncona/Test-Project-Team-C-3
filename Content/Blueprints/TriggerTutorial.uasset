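; Tutorial trigger volume that shows a timed popup message when the SideScrollerCharacter enters it.
; On overlap, the IDPopup variable selects one of four branches, each creating a new UIMessage widget, adding it to the viewport and calling its matching UIPopUp function.
; After a short delay the widget is collapsed rather than removed, and nothing in the graph prevents repeat triggering.
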(event `self.Trigger.OnComponentBeginOverlap`
  (params (OverlappedComponent :type "PrimitiveComponent Object Reference") (OtherActor :type "Actor Object Reference") (OtherComp :type "PrimitiveComponent Object Reference") (OtherBodyIndex :type Integer) (bFromSweep :type Boolean) (SweepResult :type "HitResult Structure (by ref)"))
  (cast `/Game/SideScrollerBP/Blueprints/SideScrollerCharacter` OtherActor)
  (if (== (`self.ID_Popup`) 0)
    (bind _returnvalue (`|CreateWidget` "/Game/Widget_UIMessage.Widget_UIMessage_C" (`GameplayStatics.GetPlayerController` 0)))
    (bind _output_get (set `self.Popup` _returnvalue))
    (`Widget.SetVisibility` _output_get "Visible")
    (`UserWidget.AddToViewport` _output_get 0)
    (`/Game/Widget_UIMessage.UI_PopUp_0` _output_get)
    (`KismetSystemLibrary.Delay` 5.0)
    (`Widget.SetVisibility` _output_get "Collapsed")
    (elif (== (`self.ID_Popup`) 1)
      (bind _returnvalue_2 (`|CreateWidget` "/Game/Widget_UIMessage.Widget_UIMessage_C" (`GameplayStatics.GetPlayerController` 0)))
      (bind _output_get_2 (set `self.Popup` _returnvalue_2))
      (`Widget.SetVisibility` _output_get_2 "Visible")
      (`UserWidget.AddToViewport` _output_get_2 0)
      (`/Game/Widget_UIMessage.UI_PopUp_1` _output_get_2)
      (`KismetSystemLibrary.Delay` 5.0)
      (`Widget.SetVisibility` _output_get_2 "Collapsed")
      (elif (== (`self.ID_Popup`) 2)
        (bind _returnvalue_3 (`|CreateWidget` "/Game/Widget_UIMessage.Widget_UIMessage_C" (`GameplayStatics.GetPlayerController` 0)))
        (bind _output_get_3 (set `self.Popup` _returnvalue_3))
        (`Widget.SetVisibility` _output_get_3 "Visible")
        (`UserWidget.AddToViewport` _output_get_3 0)
        (`/Game/Widget_UIMessage.UI_PopUp_2` _output_get_3)
        (`KismetSystemLibrary.Delay` 5.0)
        (`Widget.SetVisibility` _output_get_3 "Collapsed")
        (elif (== (`self.ID_Popup`) 3)
          (bind _returnvalue_4 (`|CreateWidget` "/Game/Widget_UIMessage.Widget_UIMessage_C" (`GameplayStatics.GetPlayerController` 0)))
          (bind _output_get_4 (set `self.Popup` _returnvalue_4))
          (`Widget.SetVisibility` _output_get_4 "Visible")
          (`UserWidget.AddToViewport` _output_get_4 0)
          (`/Game/Widget_UIMessage.UI_PopUp_3` _output_get_4)
          (`KismetSystemLibrary.Delay` 5.0)
          (`Widget.SetVisibility` _output_get_4 "Collapsed"))))))

(event `self.Trigger.OnComponentEndOverlap`
  (params (OverlappedComponent :type "PrimitiveComponent Object Reference") (OtherActor :type "Actor Object Reference") (OtherComp :type "PrimitiveComponent Object Reference") (OtherBodyIndex :type Integer)))

(fn `UserConstructionScript`)