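; Respawner actor that spawns an enemy of a configured class at its own transform and keeps a reference to it.
; AttemptRespawn runs on BeginPlay and spawns a replacement only when the stored enemy reference is invalid, ignoring collisions.
; CopyFromEnemy converts a placed enemy into respawner setup by adopting its class and transform, then destroying it and clearing the reference.
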(event `self.ReceiveBeginPlay`
  (`self.AttemptRespawn`))

(event `AttemptRespawn`
  (`/Engine/EditorBlueprintResources/StandardMacros.IsValid` (`self.EnemyRef`)
    (:`Is Not Valid`
      (bind _returnvalue (`|SpawnActorFromClass` (`self.EnemyClass`) (`self.GetTransform`) "AlwaysSpawn" "OverrideRootScale" null null))
      (set `self.EnemyRef` _returnvalue))))

(fn `CopyFromEnemy`
  (bind _enemytocopy (`self.EnemyToCopy`))
  (`/Engine/EditorBlueprintResources/StandardMacros.IsValid` _enemytocopy
    (:`Is Valid`
      (set `self.EnemyClass` (`GameplayStatics.GetObjectClass` _enemytocopy))
      (`self.K2_SetActorTransform` (`self.GetTransform` (`self.EnemyToCopy`)))
      (`self.K2_DestroyActor` (`self.EnemyToCopy`))
      (set `self.EnemyToCopy` null))))

(fn `UserConstructionScript`)