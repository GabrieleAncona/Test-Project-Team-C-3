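; Side-scroller trap platform that vanishes shortly after the player steps on it, then reappears.
; A Box overlap by a SideScrollerCharacter runs a delayed sequence: swap the platform material as a warning, then hide it and disable collision on platform and box.
; After a further delay, PlatformReset restores material, visibility and collision and re-arms the DoOnce gate.
; The platform never moves; the transform saved at BeginPlay is unused.
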(event `self.ReceiveBeginPlay`
  (set `self.Initial Position` (`self.GetTransform`)))

(event `self.Box.OnComponentBeginOverlap`
  (params (OverlappedComponent :type "PrimitiveComponent Object Reference") (OtherActor :type "Actor Object Reference") (OtherComp :type "PrimitiveComponent Object Reference") (OtherBodyIndex :type Integer) (bFromSweep :type Boolean) (SweepResult :type "HitResult Structure (by ref)"))
  (bind _platform (`self.platform`))
  (cast `/Game/SideScrollerBP/Blueprints/SideScrollerCharacter` OtherActor)
  (`/Engine/EditorBlueprintResources/StandardMacros.DoOnce` false :!label _label
    (:`Completed`
      (`KismetSystemLibrary.Delay` 0.2)
      (`PrimitiveComponent.SetMaterial` (`self.platform`) 0 "/Game/Geometry/Meshes/CubeMaterial.CubeMaterial")
      (`KismetSystemLibrary.Delay` 0.2)
      (`PrimitiveComponent.SetCollisionEnabled` _platform "NoCollision")
      (`PrimitiveComponent.SetCollisionEnabled` (`self.Box`) "NoCollision")
      (`SceneComponent.SetVisibility` _platform false false)
      (`KismetSystemLibrary.Delay` 2.0)
      (`self.PlatformReset`))))

(event `PlatformReset`
  (bind _platform (`self.platform`))
  (`PrimitiveComponent.SetMaterial` (`self.platform`) 0 "/Game/SideScrollerBP/Meshes/Material_001.Material_001")
  (`PrimitiveComponent.SetCollisionEnabled` _platform "QueryAndPhysics")
  (`PrimitiveComponent.SetCollisionEnabled` (`self.Box`) "QueryAndPhysics")
  (`SceneComponent.SetVisibility` _platform true false)
  (goto _label :!via `Reset`))

(fn `UserConstructionScript`)