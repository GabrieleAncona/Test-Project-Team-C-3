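; Moving platform for a side scroller that carries a jammer zone suppressing the player's time power.
; A timeline started on BeginPlay lerps the mesh from its start location by the EndPoint offset.
; While the sphere overlap flag is set, Tick blocks the character's power, clears jammer and fast effects and restores normal time.
; Leaving the sphere re-enables the power, and receiving damage destroys the platform.
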(event `self.ReceiveBeginPlay`
  (set `self.StartingPoint` (`self.K2_GetActorLocation`))
  (bind (_direction _newtrack_0) (`Timeline|PlatformAnim`)
    (:`Update`
      (`SceneComponent.K2_SetWorldLocation` (`self.StaticMesh`) (`KismetMathLibrary.VLerp` (`self.StartingPoint`) (+ (`self.StartingPoint`) (`self.EndPoint`)) _newtrack_0) false false))))

(event `self.Sphere.OnComponentBeginOverlap`
  (params (OverlappedComponent :type "PrimitiveComponent Object Reference") (OtherActor :type "Actor Object Reference") (OtherComp :type "PrimitiveComponent Object Reference") (OtherBodyIndex :type Integer) (bFromSweep :type Boolean) (SweepResult :type "HitResult Structure (by ref)"))
  (set `self.isstaying` true))

(event `self.Sphere.OnComponentEndOverlap`
  (params (OverlappedComponent :type "PrimitiveComponent Object Reference") (OtherActor :type "Actor Object Reference") (OtherComp :type "PrimitiveComponent Object Reference") (OtherBodyIndex :type Integer))
  (set `self.isstaying` false)
  (bind _asside_scroller_character (cast `/Game/SideScrollerBP/Blueprints/SideScrollerCharacter` OtherActor))
  (set `/Game/SideScrollerBP/Blueprints/SideScrollerCharacter.CanUsePower` true _asside_scroller_character))

(event `self.ReceiveTick`
  (params (DeltaSeconds :type "Float (single-precision)"))
  (bind _asside_scroller_character (cast `/Game/SideScrollerBP/Blueprints/SideScrollerCharacter` (stale `self.Sphere.OnComponentBeginOverlap` OtherActor)))
  (if (`self.isstaying`)
    (set `/Game/SideScrollerBP/Blueprints/SideScrollerCharacter.CanUsePower` false _asside_scroller_character)
    (`/Game/SideScrollerBP/Blueprints/SideScrollerCharacter.Rimuovi Effetto Jammer` _asside_scroller_character)
    (`/Game/SideScrollerBP/Blueprints/SideScrollerCharacter.Rimuovi Effetto fast` _asside_scroller_character)
    (`/Game/SideScrollerBP/Blueprints/SideScrollerCharacter.SetNormalTime` _asside_scroller_character)))

(event `Receive Damage`
  (`self.K2_DestroyActor`))

(fn `UserConstructionScript`)