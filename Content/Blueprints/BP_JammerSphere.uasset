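; A jammer sphere actor that blocks the player's powers in the side-scroller while the player is inside its overlap sphere.
; On entry it sets IsPowerJammed on the SideScrollerCharacter, calls its functions to remove jammer and fast effects and restore normal time, and turns Sphere1 grey through a dynamic material.
; Leaving clears the flag and turns that material blue.
; Receiving damage destroys the actor.
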(event `self.Sphere.OnComponentEndOverlap`
  (params (OverlappedComponent :type "PrimitiveComponent Object Reference") (OtherActor :type "Actor Object Reference") (OtherComp :type "PrimitiveComponent Object Reference") (OtherBodyIndex :type Integer))
  (if (== OtherActor (`GameplayStatics.GetPlayerPawn` 0))
    (`MaterialInstanceDynamic.SetVectorParameterValue` (stale `self.Sphere.OnComponentBeginOverlap` _returnvalue) "Color" (struct :`R` 0.028426 :`G` 0.045186 :`B` 0.617207 :`A` 1.0))
    (bind _asside_scroller_character (cast `/Game/SideScrollerBP/Blueprints/SideScrollerCharacter` OtherActor))
    (set `/Game/SideScrollerBP/Blueprints/SideScrollerCharacter.IsPowerJammed` false _asside_scroller_character)))

(event `self.Sphere.OnComponentBeginOverlap`
  (params (OverlappedComponent :type "PrimitiveComponent Object Reference") (OtherActor :type "Actor Object Reference") (OtherComp :type "PrimitiveComponent Object Reference") (OtherBodyIndex :type Integer) (bFromSweep :type Boolean) (SweepResult :type "HitResult Structure (by ref)"))
  (if (== OtherActor (`GameplayStatics.GetPlayerPawn` 0))
    (bind _returnvalue (`PrimitiveComponent.CreateDynamicMaterialInstance` (`self.Sphere1`) 0 "/Game/Shaders/InstanceMaterial.InstanceMaterial" "None"))
    (`MaterialInstanceDynamic.SetVectorParameterValue` _returnvalue "Color" (struct :`R` 0.166667 :`G` 0.166667 :`B` 0.166667 :`A` 1.0))
    (bind _asside_scroller_character (cast `/Game/SideScrollerBP/Blueprints/SideScrollerCharacter` OtherActor))
    (set `/Game/SideScrollerBP/Blueprints/SideScrollerCharacter.IsPowerJammed` true _asside_scroller_character)
    (`/Game/SideScrollerBP/Blueprints/SideScrollerCharacter.Rimuovi Effetto Jammer` _asside_scroller_character)
    (`/Game/SideScrollerBP/Blueprints/SideScrollerCharacter.Rimuovi Effetto fast` _asside_scroller_character)
    (`/Game/SideScrollerBP/Blueprints/SideScrollerCharacter.SetNormalTime` _asside_scroller_character)))

(event `Receive Damage`
  (`self.K2_DestroyActor`))

(fn `UserConstructionScript`)