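; Interactive door actor that the player opens and closes with the E key while near it.
; Overlapping the Box enables input from player controller 0, and leaving it disables input, with no check on which actor overlaps.
; E flips DoorClosed and plays or reverses the Opening_door timeline, whose OpenClose track sets the Door's yaw as an absolute world rotation.
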(event `self.Box.OnComponentBeginOverlap`
  (params (OverlappedComponent :type "PrimitiveComponent Object Reference") (OtherActor :type "Actor Object Reference") (OtherComp :type "PrimitiveComponent Object Reference") (OtherBodyIndex :type Integer) (bFromSweep :type Boolean) (SweepResult :type "HitResult Structure (by ref)"))
  ;[1 1 1] Enable/Disable Input
  (`self.EnableInput` (`GameplayStatics.GetPlayerController` 0)))

(event `self.Box.OnComponentEndOverlap`
  (params (OverlappedComponent :type "PrimitiveComponent Object Reference") (OtherActor :type "Actor Object Reference") (OtherComp :type "PrimitiveComponent Object Reference") (OtherBodyIndex :type Integer))
  ;[1 1 1] Enable/Disable Input
  (`self.DisableInput` (`GameplayStatics.GetPlayerController` 0)))

(event `Key|E`
  (params (Key :type "Key Structure"))
  ;[1 1 1] Opening/Closing Door
  (:`Pressed`
    (if (`self.Door_Closed`)
      (set `self.Door_Closed` false)
      (bind (_direction _open_close) (`Timeline|Opening_door` :!label _label)
        (:`Update`
          (`SceneComponent.K2_SetWorldRotation` (`self.Door`) (`KismetMathLibrary.MakeRotator` 0.0 0.0 _open_close) false false)))
      (else
        (set `self.Door_Closed` true)
        (goto _label :!via `Reverse`)))))

(fn `UserConstructionScript`)