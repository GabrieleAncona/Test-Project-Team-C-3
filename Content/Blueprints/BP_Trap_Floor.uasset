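; BP_Trap_Floor is a floor trap that damages a SideScrollerCharacter overlapping its Box component.
; On overlap it shows the character's BloodHud for half a second, then hides it and subtracts Damage from CurrentHP.
; At zero HP or below it destroys player character 0, rather than the overlapping reference.
; A parallel Sequence branch increments HitPlayerCount on SideScrollerGameMode immediately, without waiting for the delay.
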(event `self.Box.OnComponentBeginOverlap`
  (params (OverlappedComponent :type "PrimitiveComponent Object Reference") (OtherActor :type "Actor Object Reference") (OtherComp :type "PrimitiveComponent Object Reference") (OtherBodyIndex :type Integer) (bFromSweep :type Boolean) (SweepResult :type "HitResult Structure (by ref)"))
  (bind _asside_scroller_character (cast `/Game/SideScrollerBP/Blueprints/SideScrollerCharacter` OtherActor))
  (`|ExecutionSequence`
    (:`then_0`
      (bind _bloodhud (`/Game/SideScrollerBP/Blueprints/SideScrollerCharacter.BloodHud` _asside_scroller_character))
      (`Widget.SetVisibility` _bloodhud "Visible")
      (`KismetSystemLibrary.Delay` 0.5)
      (`Widget.SetVisibility` _bloodhud "Collapsed")
      (bind _output_get (set `/Game/SideScrollerBP/Blueprints/SideScrollerCharacter.CurrentHP` (- (`/Game/SideScrollerBP/Blueprints/SideScrollerCharacter.CurrentHP` _asside_scroller_character) (`self.Damage`)) _asside_scroller_character))
      (if (<= _output_get 0.0)
        (`self.K2_DestroyActor` (`GameplayStatics.GetPlayerCharacter` 0))))
    (:`then_1`
      (bind _asside_scroller_game_mode (cast `/Game/SideScrollerBP/Blueprints/SideScrollerGameMode` (`GameplayStatics.GetGameMode`)))
      (set `/Game/SideScrollerBP/Blueprints/SideScrollerGameMode.HitPlayerCount` (+ (`/Game/SideScrollerBP/Blueprints/SideScrollerGameMode.HitPlayerCount` _asside_scroller_game_mode) 1) _asside_scroller_game_mode))))

(fn `UserConstructionScript`)